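; BP_Enemy is an enemy character Blueprint that handles its death and keeps an on-actor health bar in sync.
; On death it plays a melee death montage on the mesh and destroys the actor when the montage completes, blends out or hits a notify end.
; Health change events push the health-to-max ratio into the WB_HealthBar widget held by its HealthBar component.
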(event EventOnHealthChange
  (params (Health :type Float%20%28single-precision%29) (MaxHealth :type Float%20%28single-precision%29))
  ;[1 1 1] When Health Change we udpate the health UI
  (Default|SetPercentage (.AsWB%20Health%20Bar (Utilities|Casting|CastToWB_HealthBar (UserInterface|GetUserWidgetObject (Variables|Default|GetHealthBar)))) (/ Health MaxHealth)))

(event Collision|EventActorBeginOverlap
  (params (OtherActor :type Actor%20Object%20Reference))
  (|CallParentFunction OtherActor) ; This node is disabled and will not be called.\nDrag off pins to build functionality.
)

(event EventOnDeath
  ;[1 1 1] Death Animation
  (Animation|Montage|PlayMontage (Variables|Character|GetMesh) "/Game/Project/Characters/Animations/AnimationMontages/AM_MeleeOnDeath.AM_MeleeOnDeath"
    (:OnCompleted
      _)
    (:OnBlendOut
      _)
    (:OnNotifyEnd
      _))
  (Actor|DestroyActor))

(fn ConstructionScript
  (|CallParentFunction))