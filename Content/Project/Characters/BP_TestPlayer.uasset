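; Player character Blueprint built on the Gameplay Ability System, granting melee, health regen and dash abilities at BeginPlay and activating them through Try events.
; Sword overlaps with hostiles and dash collisions reported from C++ send tagged gameplay events for damage.
; Tick tracks acceleration and airborne state, while other events update health and mana globes, pass stun to the animation instance, apply impulses and destroy the actor after its death montage.
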(event OnComponentBeginOverlap(SwordCollisionCapsule)
  (params (OverlappedComponent :type Primitive%20Component%20Object%20Reference) (OtherActor :type Actor%20Object%20Reference) (OtherComp :type Primitive%20Component%20Object%20Reference) (OtherBodyIndex :type Integer) (bFromSweep :type Boolean) (SweepResult :type Hit%20Result%20Structure%20%28by%20ref%29))
  ;[1 1 1] Melee Ability
  (bind _returnvalue (Class|BasicChar|IsOtherHostile (.AsBasic%20Char%20BP (Utilities|Casting|CastToBasicChar_BP OtherActor))))
  (if _returnvalue
    (Ability|SendGameplayEventtoActor self "(TagName=\"Skill.Melee.DealDamage\")" (Utilities|Struct|MakeGameplayEventData "" 0 OtherActor))))

(event Custom|PushCharacter
  (params (Direction :type Vector) (Strenght :type Float%20%28single-precision%29) (ImpulsedTarget :type Basic%20Char%20BP%20Object%20Reference) (Stun%20Duration :type Float%20%28single-precision%29) (IsStunActive :type Boolean))
  ;[1 1 1] Dash Impulse
  (Variables|Movement|SetOriginalFriction 0.0)
  (Physics|AddImpulse (Variables|/Script/Engine.Character|GetCharacterMovement ImpulsedTarget) (* Direction Strenght) true)
  (if (and (> Stun%20Duration 0.0) IsStunActive)
    (Class|BasicChar|HitStun Stun%20Duration))
  (Variables|Movement|SetOriginalFriction (Variables|Movement|GetOriginalFriction)))

(event Custom|TryHealthRegen
  ;[1 1 1] Gameplay Abilities Events
  (Class|BasicChar|CharacterActivateAbilitybyClass "/Game/Project/GameplayAbilities/HealthRegen/GA_HealthRegen.GA_HealthRegen_C" false))

(event Custom|OriginalFrictionSetUp
  ;[1 1 1] Original Friction Set Up (Will be used in on air dashes animations to not slide through the floor )
  (Variables|Movement|SetOriginalFriction (Variables|/Script/Engine.CharacterMovementComponent|GetGroundFriction (Variables|Character|GetCharacterMovement))))

(event Custom|TryDash
  ;[1 1 1] Gameplay Abilities Events
  (Class|BasicChar|CharacterActivateAbilitybyClass "/Game/Project/GameplayAbilities/Dash/GA_Dash.GA_Dash_C" false))

(event Custom|TryMeleeAttack
  ;[1 1 1] Gameplay Abilities Events
  (Class|BasicChar|CharacterActivateAbilitybyClass "/Game/Project/GameplayAbilities/Melee/GA_Melee.GA_Melee_C" false))

(event EventBeginPlay
  ;[1 1 1] Variables Set Up
  (CallFunction|OriginalFrictionSetUp)
  ;[1 1 1] We acquire the abilities at the begining for later use
  (Class|BasicChar|AquireAbility "/Game/Project/GameplayAbilities/Melee/GA_Melee.GA_Melee_C")
  (Class|BasicChar|AquireAbility "/Game/Project/GameplayAbilities/HealthRegen/GA_HealthRegen.GA_HealthRegen_C")
  (Class|BasicChar|AquireAbility "/Game/Project/GameplayAbilities/Dash/GA_Dash.GA_Dash_C"))

(event EventOnDeath
  ;[1 1 1] State Events
  (Animation|Montage|PlayMontage (Variables|Character|GetMesh) "/Game/Project/Characters/Animations/AnimationMontages/AM_MeleeOnDeath.AM_MeleeOnDeath" 1.0 0.0 ""
    (:OnBlendOut
      (Actor|DestroyActor))))

(event EventOnHealthChange
  (params (Health :type Float%20%28single-precision%29) (MaxHealth :type Float%20%28single-precision%29))
  ;[1 1 1] UI Update
  (Default|SetPercentge (Variables|/Game/Project/UI/PrimaryUI.PrimaryUI_C|GetHealthGlassBall (Variables|/Game/Project/Controllers/PlayerControllerBase_BP.PlayerControllerBase_BP_C|GetMainUI (.AsPlayer%20Controller%20Base%20BP (Utilities|Casting|CastToPlayerControllerBase_BP (Pawn|GetController))))) (/ Health MaxHealth)))

(event EventOnManaChange
  (params (Mana :type Float%20%28single-precision%29) (MaxMana :type Float%20%28single-precision%29))
  ;[1 1 1] UI Update
  (Default|SetPercentge (Variables|/Game/Project/UI/PrimaryUI.PrimaryUI_C|GetManaGlassBall (Variables|/Game/Project/Controllers/PlayerControllerBase_BP.PlayerControllerBase_BP_C|GetMainUI (.AsPlayer%20Controller%20Base%20BP (Utilities|Casting|CastToPlayerControllerBase_BP (Pawn|GetController))))) (/ Mana MaxMana)))

(event EventTick
  (params (DeltaSeconds :type Float%20%28single-precision%29))
  (bind _charactermovement (Variables|Character|GetCharacterMovement))
  ;[1 1 1] Acceleration Set Up
  (if (> (Math|Vector|VectorLength (Pawn|Components|CharacterMovement|GetCurrentAcceleration _charactermovement)) 0.0)
    (Variables|State|SetIsAccelerating true)
    (else
      (Variables|State|SetIsAccelerating false)))
  ;[1 1 1] Is In Air Set Up and if is jumping, can´t accelerate
  (if (AI|Components|NavMovement|IsFalling _charactermovement)
    (Variables|State|SetIsInAir true)
    (Variables|State|SetIsAccelerating false)
    (else
      (Variables|State|SetIsInAir false))))

(event EventDashCollisionEnemies
  ;[1 1 1] Event Called from c++ when we overlapp an enemy dashing, then we send the gameplay event data to the instigator to apply the damage to the dashed enemies
  (bind _dashedenemies (Class|BasicChar|GetDashedEnemies))
  (for _array_element _dashedenemies
    _)
  (Ability|SendGameplayEventtoActor self "(TagName=\"Skill.Dash.DealDamage\")" (Utilities|Struct|MakeGameplayEventData "" 0 _array_element 0 0 "()" "(GameplayTags=)" "(GameplayTags=)" 0.0 (Ability|TargetData|AbilityTargetDatafromActor _array_element))))

(event EventOnStun
  ;[1 1 1] State Events
  (Variables|State|SetIsStun true)
  (bind _asanim3 (Utilities|Casting|CastToANIM3 (Components|SkeletalMesh|GetAnimInstance (Variables|Character|GetMesh))))
  (Variables|/Game/Project/Characters/Animations/Animations_Bps/ANIM3.ANIM3_C|SetIsStun _asanim3 true))

(event EventOnEndStun
  ;[1 1 1] State Events
  (Variables|State|SetIsStun false)
  (bind _asanim3 (Utilities|Casting|CastToANIM3 (Components|SkeletalMesh|GetAnimInstance (Variables|Character|GetMesh))))
  (Variables|/Game/Project/Characters/Animations/Animations_Bps/ANIM3.ANIM3_C|SetIsStun _asanim3 false))

(fn ConstructionScript)

(fn SetCapsuleCollision
  (params (DashCollisionChanel :type ECollisionChannel%20Enum :default "ECC_WorldStatic") (CollisionResponse :type ECollisionResponse%20Enum :default "ECR_Ignore"))
  (Collision|SetCollisionResponsetoChannel (Variables|Default|GetCapsuleComponent) DashCollisionChanel CollisionResponse))