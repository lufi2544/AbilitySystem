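; Base player controller that creates the primary UI on BeginPlay and routes player input to the controlled pawn.
; Movement axes push the pawn along the camera manager's forward and right vectors, using the full camera rotation including pitch.
; Look axes add pitch and yaw input to the pawn.
; Jump casts the pawn to Character, while melee attack casts it to BP_MeleePlayer, tying that action to that class.
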(event EventBeginPlay
  (bind _returnvalue (UserInterface|CreateWidget "/Game/Project/UI/PrimaryUI.PrimaryUI_C"))
  (Variables|Default|SetMainUI _returnvalue)
  (UserInterface|Viewport|AddtoViewport _returnvalue 0))

(event Input|ActionEvents|InputActionJump
  (params (Key :type Key%20Structure :default "None"))
  ;[0 0.7209 1] Movement Set Up
  (:Pressed
    (Character|Jump (.AsCharacter (Utilities|Casting|CastToCharacter (Pawn|GetControlledPawn))))))

(event Input|ActionEvents|InputActionAttackMelee
  (params (Key :type Key%20Structure :default "None"))
  (:Pressed
    (Default|MeleeAttack (.AsBP%20Melee%20Player (Utilities|Casting|CastToBP_MeleePlayer (Pawn|GetControlledPawn))))))

(event Input|AxisEvents|InputAxisMoveForward
  (params (AxisValue :type Float%20%28single-precision%29))
  ;[0 0.7209 1] Movement Set Up
  (Pawn|Input|AddMovementInput (Pawn|GetControlledPawn) (Math|Vector|GetForwardVector (Camera|GetCameraRotation (Variables|Default|GetPlayerCameraManager))) AxisValue false))

(event Input|AxisEvents|InputAxisMoveRight
  (params (AxisValue :type Float%20%28single-precision%29))
  ;[0 0.7209 1] Movement Set Up
  (Pawn|Input|AddMovementInput (Pawn|GetControlledPawn) (Math|Vector|GetRightVector (Camera|GetCameraRotation (Variables|Default|GetPlayerCameraManager))) AxisValue false))

(event Input|AxisEvents|InputAxisLookingRight
  (params (AxisValue :type Float%20%28single-precision%29))
  ;[0 0.7209 1] Movement Set Up
  (Pawn|Input|AddControllerYawInput (Pawn|GetControlledPawn) AxisValue))

(event Input|AxisEvents|InputAxisLookingUp
  (params (AxisValue :type Float%20%28single-precision%29))
  ;[0 0.7209 1] Movement Set Up
  (Pawn|Input|AddControllerPitchInput (Pawn|GetControlledPawn) AxisValue))

(fn ConstructionScript)