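; PlayerControllerBase_BP is a player controller that turns input into movement, look, jump and melee actions on the possessed pawn.
; Move axes add movement input along the camera manager's full-rotation forward and right vectors, while look axes feed pitch and yaw.
; Jump casts the pawn to Character, and AttackMelee casts it to PlayerChar_BP to play the Melee montage on its mesh, with no hit logic here.
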(event Input|ActionEvents|InputActionJump
  (params (Key :type Key%20Structure :default "None"))
  ;[0 0.7209 1] Movement Set Up
  (:Pressed
    (Character|Jump (.AsCharacter (Utilities|Casting|CastToCharacter (Pawn|GetControlledPawn))))))

(event Input|ActionEvents|InputActionAttackMelee
  (params (Key :type Key%20Structure :default "None"))
  (:Pressed
    (Animation|Montage|PlayMontage (Variables|/Script/Engine.Character|GetMesh (.AsPlayer%20Char%20BP (Utilities|Casting|CastToPlayerChar_BP (Pawn|GetControlledPawn)))) "/Game/Animation_BPs/Melee.Melee")))

(event Input|AxisEvents|InputAxisMoveForward
  (params (AxisValue :type Float%20%28single-precision%29))
  ;[0 0.7209 1] Movement Set Up
  (Pawn|Input|AddMovementInput (Pawn|GetControlledPawn) (Math|Vector|GetForwardVector (Camera|GetCameraRotation (Variables|Default|GetPlayerCameraManager))) AxisValue false))

(event Input|AxisEvents|InputAxisMoveRight
  (params (AxisValue :type Float%20%28single-precision%29))
  ;[0 0.7209 1] Movement Set Up
  (Pawn|Input|AddMovementInput (Pawn|GetControlledPawn) (Math|Vector|GetRightVector (Camera|GetCameraRotation (Variables|Default|GetPlayerCameraManager))) AxisValue false))

(event Input|AxisEvents|InputAxisLookingRight
  (params (AxisValue :type Float%20%28single-precision%29))
  ;[0 0.7209 1] Movement Set Up
  (Pawn|Input|AddControllerYawInput (Pawn|GetControlledPawn) AxisValue))

(event Input|AxisEvents|InputAxisLookingUp
  (params (AxisValue :type Float%20%28single-precision%29))
  ;[0 0.7209 1] Movement Set Up
  (Pawn|Input|AddControllerPitchInput (Pawn|GetControlledPawn) AxisValue))

(fn ConstructionScript)