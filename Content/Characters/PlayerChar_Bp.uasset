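; Player character Blueprint that tracks movement state flags every Tick.
; IsAccelerating is true when the CharacterMovement component's current acceleration on the Y axis is non-zero; other axes are ignored.
; IsInAir mirrors the component's IsFalling check and forces IsAccelerating to false while airborne.
; The construction script is empty, and the graph only sets these flags without applying any movement.
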(event EventTick
  (params (DeltaSeconds :type Float%20%28single-precision%29))
  (bind _charactermovement (Variables|Character|GetCharacterMovement))
  ;[1 1 1] Acceleration Set Up
  (if (!= (.y (Pawn|Components|CharacterMovement|GetCurrentAcceleration _charactermovement)) 0.0)
    (Variables|Default|SetIsAccelerating true)
    (else
      (Variables|Default|SetIsAccelerating false)))
  ;[1 1 1] Is In Air Set Up and if is jumping, can´t accelerate
  (if (AI|Components|NavMovement|IsFalling _charactermovement)
    (Variables|Default|SetIsInAir true)
    (Variables|Default|SetIsAccelerating false)
    (else
      (Variables|Default|SetIsInAir false))))

(fn ConstructionScript)